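; Betrayal condition for a unit, met when its current health is at or below HPThreshold.
; Registering stores the owner unit and binds an event to its health-changed delegate, unregistering unbinds it, and both return false.
; The generated health-changed function is empty.
; Its logic to recheck, switch the unit to Player affiliation and recolor the health bar is disconnected and never runs.
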(fn CheckCondition
  (params (Unit :type LFP%20Tactics%20Unit%20Object%20Reference))
  (return (<= (Class|LFPTacticsUnit|GetCurrentHealth Unit) (Variables|Default|GetHPThreshold))))

(fn RegisterCondition
  (params (Unit :type LFP%20Tactics%20Unit%20Object%20Reference))
  (Variables|Default|SetOwnerUnit Unit)
  (EventDispatchers|BindEventtoOnHealthChangedDelegate Unit (EventDispatchers|CreateEvent :!event BPBConditionHPLackAutoGenFunc))
  (return false))

(fn BPBConditionHPLackAutoGenFunc
  (params (CurrentHealth :type Integer) (MaxHealth :type Integer)))

(fn UnRegisterCondition
  (params (Unit :type LFP%20Tactics%20Unit%20Object%20Reference))
  (EventDispatchers|UnbindEventfromOnHealthChangedDelegate Unit (EventDispatchers|CreateEvent :!event BPBConditionHPLackAutoGenFunc))
  (return false))