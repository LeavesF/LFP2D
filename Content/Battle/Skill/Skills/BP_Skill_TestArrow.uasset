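; Test arrow skill for grid battles that deals typed damage to the unit on the target tile.
; CanReleaseFrom adds to the parent check by refreshing range from the caster tile and requiring an opposing unit at a listed coordinate.
; CanExecute, hatred value and range getter just return parent results.
; A six-direction hex line scan for enemies and an extra CanExecute range check remain as disconnected, unexecuted logic.
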(event EventExecute
  (params (TargetTile :type LFP%20Hex%20Tile%20Object%20Reference))
  (Utilities|IsValid TargetTile
    (:Is%20Valid
      (bind _returnvalue (Class|LFPHexTile|GetUnitonTile TargetTile))
      (Utilities|IsValid _returnvalue
        (:Is%20Valid
          (Class|LFPTacticsUnit|ReceiveTypedDamage _returnvalue (Variables|Default|GetDamage)))))))

(fn CanExecute
  (params (TargetTile :type LFP%20Hex%20Tile%20Object%20Reference))
  (bind _returnvalue (|CallParentFunction TargetTile))
  (return _returnvalue))

(fn CanReleasefrom
  (params (CasterTile :type LFP%20Hex%20Tile%20Object%20Reference) (TargetTile :type LFP%20Hex%20Tile%20Object%20Reference))
  (bind _returnvalue (|CallParentFunction CasterTile TargetTile))
  (if _returnvalue
    (Variables|Default|SetCurReleaseTile CasterTile)
    (Class|LFPSkillBase|UpdateSkillRange)
    (bind _returnvalue_2 (Class|LFPHexTile|GetUnitonTile TargetTile))
    (Utilities|IsValid _returnvalue_2
      (:Is%20Valid
        (if (not (Utilities|Enum|Equal(Enum) (Class|LFPTacticsUnit|GetAffiliation _returnvalue_2) (Class|LFPTacticsUnit|GetAffiliation (Variables|Default|GetOwner))))
          (bind _returnvalue_3 (Class|LFPHexTile|GetCoordinates TargetTile))
          (for _array_element (Variables|Default|GetReleaseRangeInGridCoords)
            (if (and (== (.q _returnvalue_3) (.q _array_element)) (== (.r _returnvalue_3) (.r _array_element)))
              (return true)))
          (return false))))
    (else
      (return false))))

(fn CalculateHatredValue
  (params (Caster :type LFP%20Tactics%20Unit%20Object%20Reference) (Target :type LFP%20Tactics%20Unit%20Object%20Reference))
  (return (|CallParentFunction 0 0)))

(fn GetReleaseRangeinGrid
  (bind _returnvalue (|CallParentFunction))
  (return _returnvalue))